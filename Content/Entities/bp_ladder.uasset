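; Climbable ladder actor that the player can climb while overlapping its collision box.
; The construction script stacks a configurable number of section meshes, spaced by the mesh's height.
; It then sizes and centers the climb box over the stack, with tunable size and offsets.
; Overlap begin and end on that box toggle climbing on bp_ZPlayer, passing the ladder as reference.
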(event `self.ladderClimbCollision.OnComponentBeginOverlap`
  (params (OverlappedComponent :type "PrimitiveComponent Object Reference") (OtherActor :type "Actor Object Reference") (OtherComp :type "PrimitiveComponent Object Reference") (OtherBodyIndex :type Integer) (bFromSweep :type Boolean) (SweepResult :type "HitResult Structure (by ref)"))
  (bind _asbp_zplayer (cast `/Game/Characters/Blueprints/bp_ZPlayer` OtherActor))
  (`/Game/Characters/Blueprints/bp_ZPlayer.toggleClimbing` _asbp_zplayer true self))

(event `self.ladderClimbCollision.OnComponentEndOverlap`
  (params (OverlappedComponent :type "PrimitiveComponent Object Reference") (OtherActor :type "Actor Object Reference") (OtherComp :type "PrimitiveComponent Object Reference") (OtherBodyIndex :type Integer))
  (bind _asbp_zplayer (cast `/Game/Characters/Blueprints/bp_ZPlayer` OtherActor))
  (`/Game/Characters/Blueprints/bp_ZPlayer.toggleClimbing` _asbp_zplayer false self))

(fn `UserConstructionScript`
  (`|ExecutionSequence`
    (:`then_0`
      (set `self.sectionHeight` (* (.z (`.BoxExtent` (`KismetMathLibrary.BreakBoxSphereBounds` (`StaticMesh.GetBounds` (`self.ladderSectionMesh`))))) 2.0)))
    (:`then_1`
      (for _index (range (`self.ladderPieces`))
        (bind _returnvalue (`AddComponent|NODE_AddStaticMeshComponent-0` :`RelativeTransform` (`KismetMathLibrary.MakeTransform` (`KismetMathLibrary.MakeVector` 0.0 0.0 (* _index (`self.sectionHeight`))) (struct) (1.0 0.6 1.0))))
        (`StaticMeshComponent.SetStaticMesh` _returnvalue (`self.ladderSectionMesh`))))
    (:`then_2`
      (`BoxComponent.SetBoxExtent` (`self.ladderClimbCollision`) (`KismetMathLibrary.MakeVector` (`self.ladderCollisionSizeX`) (`self.ladderCollisionSizeY`) (- (/ (* (`self.ladderPieces`) (`self.sectionHeight`)) 2.0) (`self.ladderCollisionSizeOffsetZ`))) true)
      (`SceneComponent.K2_SetRelativeLocation` (`self.ladderClimbCollision`) (`KismetMathLibrary.MakeVector` (`self.xOffset`) (`self.yOffset`) (+ (.z (break `Box` (`StaticMesh.GetBoundingBox` (`self.ladderSectionMesh`)))) (/ (* (`self.ladderPieces`) (`self.sectionHeight`)) 2.0))) false false))))