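; Interactable button that opens the sliding doors whose DoorID matches its ButtonID.
; CharInteracted searches all Bp_slidingDoor actors and calls OpenDoor on the first match, or on every match when CanControlMultiple is set.
; Box overlap events show and hide the bp_ZPlayer's InteractText and track IsPlayerClose, which CharInteracted does not check.
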(event `self.CharInteracted`
  (if (not (`self.canControlMultiple`))
    (bind _outactors (`GameplayStatics.GetAllActorsOfClass` "/Game/Entities/bp_slidingDoor.bp_slidingDoor_C"))
    (for _array_element _outactors
      (if (== (`/Game/Entities/bp_slidingDoor.doorID` _array_element) (`self.buttonID`))
        (`/Game/Entities/bp_slidingDoor.OpenDoor` _array_element)
        (break)))
    (else
      (bind _outactors_2 (`GameplayStatics.GetAllActorsOfClass` "/Game/Entities/bp_slidingDoor.bp_slidingDoor_C"))
      (for _array_element_2 _outactors_2
        (if (== (`/Game/Entities/bp_slidingDoor.doorID` _array_element_2) (`self.buttonID`))
          (`/Game/Entities/bp_slidingDoor.OpenDoor` _array_element_2))))))

(event `self.Box.OnComponentBeginOverlap`
  (params (OverlappedComponent :type "PrimitiveComponent Object Reference") (OtherActor :type "Actor Object Reference") (OtherComp :type "PrimitiveComponent Object Reference") (OtherBodyIndex :type Integer) (bFromSweep :type Boolean) (SweepResult :type "HitResult Structure (by ref)"))
  (if (not (`self.isPlayerClose`))
    (bind _asbp_zplayer (cast `/Game/Characters/Blueprints/bp_ZPlayer` OtherActor))
    (`Widget.SetVisibility` (`/Game/Characters/Blueprints/bp_ZPlayer.InteractText` _asbp_zplayer) "Visible")
    (set `self.isPlayerClose` true)))

(event `self.Box.OnComponentEndOverlap`
  (params (OverlappedComponent :type "PrimitiveComponent Object Reference") (OtherActor :type "Actor Object Reference") (OtherComp :type "PrimitiveComponent Object Reference") (OtherBodyIndex :type Integer))
  (if (`self.isPlayerClose`)
    (bind _asbp_zplayer (cast `/Game/Characters/Blueprints/bp_ZPlayer` OtherActor))
    (`Widget.SetVisibility` (`/Game/Characters/Blueprints/bp_ZPlayer.InteractText` _asbp_zplayer) "Hidden")
    (set `self.isPlayerClose` false)))

(fn `UserConstructionScript`)