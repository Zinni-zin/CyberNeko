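; Swingable rope actor that the player grabs, with support for time rewind.
; Construction places RopeEnd at a configurable location with rewind inactive; capsule overlap by a ZPlayer notifies the player and activates the ACTimeRewind component.
; Swing pushes RopeEnd with physics impulses along supplied forward and right vectors by input sign, returning forward/backward swing state.
; Rewind relays requests to the component, while TimerStopped is an empty stub.
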(event `self.ReceiveBeginPlay`)

(event `self.Capsule.OnComponentBeginOverlap`
  (params (OverlappedComponent :type "PrimitiveComponent Object Reference") (OtherActor :type "Actor Object Reference") (OtherComp :type "PrimitiveComponent Object Reference") (OtherBodyIndex :type Integer) (bFromSweep :type Boolean) (SweepResult :type "HitResult Structure (by ref)"))
  (bind _aszplayer (cast `ZPlayer` OtherActor))
  (message `CharacterActions.CharGrabbedRope` _aszplayer self)
  (set `AC_TimeRewind.m_isActive` true (`self.AC_TimeRewind`)))

(fn `rewind`
  (params (isRewinding :type Boolean))
  (message `CharacterActions.TimeRewind` (`self.AC_TimeRewind`) isRewinding 0.0))

(fn `Swing`
  (params (`X Value` :type "Float (double-precision)") (`Y Value` :type "Float (double-precision)") (`Forward Vec` :type "Vector Structure") (RightVec :type "Vector Structure") (`Swing Impulse` :type "Float (double-precision)"))
  (returns (isSwingingForward :type Boolean) (isSwingingBackward :type Boolean))
  (`|ExecutionSequence`
    (:`then_0`
      (if (> (`local.Y Value`) 0.0)
        ;[0.009047 0.07275 1] Move Forward
        (`PrimitiveComponent.AddImpulse` (`self.RopeEnd`) (* (`KismetMathLibrary.Normal` (`local.Forward Vec`)) (`local.Swing Impulse`)) "None" false)
        (set `self.isMovingForward` true)
        (set `self.isMovingBackward` false)
        (elif (< (`local.Y Value`) 0.0)
          ;[0.009047 0.07275 1] Move Back
          (`PrimitiveComponent.AddImpulse` (`self.RopeEnd`) (* (`KismetMathLibrary.Normal` (`local.Forward Vec`)) (* (`local.Swing Impulse`) -1.0)) "None" false)
          (set `self.isMovingForward` false)
          (set `self.isMovingBackward` true))))
    (:`then_1`
      (if (> (`local.X Value`) 0.0)
        ;[0.4755 0.1303 1] Move Right
        (`PrimitiveComponent.AddImpulse` (`self.RopeEnd`) (* (`KismetMathLibrary.Normal` (`local.RightVec`)) (`local.Swing Impulse`)) "None" false)
        (elif (< (`local.X Value`) 0.0)
          ;[0.4755 0.1303 1] Move Left
          (`PrimitiveComponent.AddImpulse` (`self.RopeEnd`) (* (`KismetMathLibrary.Normal` (`local.RightVec`)) (* (`local.Swing Impulse`) -1.0)) "None" false))))
    (:`then_2`
      (return (`self.isMovingForward`) (`self.isMovingBackward`)))))

(fn `timerStopped`
  (params (time :type "Float (double-precision)")))

(fn `UserConstructionScript`
  (`SceneComponent.K2_SetRelativeLocation` (`self.RopeEnd`) (`self.ropeEndLocation`) false false)
  (set `AC_TimeRewind.m_isActive` false (`self.AC_TimeRewind`)))