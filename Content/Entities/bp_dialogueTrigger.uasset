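; One-shot dialogue trigger that pauses the game and shows a sequence of text lines when the player overlaps it, if the game instance allows dialogue.
; It registers itself and its Id on the player; NextDialogue advances the lines, then removes the widget and unpauses.
; With an input action set, it waits tick by tick for key mappings, then replaces [keyname] with the bound keyboard key before creating the widget.
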(event `self.ReceiveBeginPlay`
  (`/Engine/EditorBlueprintResources/StandardMacros.IsValid` (`self.InputToDisplay`)
    (:`Is Valid`
      (`self.ChangeTextToDisplayKey`))
    (:`Is Not Valid`
      (bind _returnvalue (`|CreateWidget` "/Game/GUI/wbp_dialogue.wbp_dialogue_C"))
      (bind _output_get (set `self.DialogueGUI` _returnvalue))
      (`TextBlock.SetText` (`/Game/GUI/wbp_dialogue.txt_dialogue` _output_get) (`|GetArrayItem` (`self.dialogueText`) (`self.dialogueIndex`))))))

(event `self.Trigger.OnComponentBeginOverlap`
  (params (OverlappedComponent :type "PrimitiveComponent Object Reference") (OtherActor :type "Actor Object Reference") (OtherComp :type "PrimitiveComponent Object Reference") (OtherBodyIndex :type Integer) (bFromSweep :type Boolean) (SweepResult :type "HitResult Structure (by ref)"))
  (bind _asbp_z_game_instance (cast `/Game/Misc/bp_zGameInstance` (`GameplayStatics.GetGameInstance`)))
  (if (and (not (`self.hasBeenActivated`)) (`/Game/Misc/bp_zGameInstance.canShowDialogue` _asbp_z_game_instance))
    (bind _asbp_zplayer (cast `/Game/Characters/Blueprints/bp_ZPlayer` OtherActor))
    (set `/Game/Characters/Blueprints/bp_ZPlayer.currentDialogue` self _asbp_zplayer)
    (set `/Game/Characters/Blueprints/bp_ZPlayer.lastDialogueActivated_ID` (`self.id`) _asbp_zplayer)
    (`UserWidget.AddToViewport` (`self.DialogueGUI`) 0)
    (set `self.hasBeenActivated` true)
    (`GameplayStatics.SetGamePaused` true)
    (`WidgetBlueprintLibrary.SetInputMode_GameAndUIEx` (`GameplayStatics.GetPlayerController` 0) (`self.DialogueGUI`))
    (set `self.isActive` true)))

(event `Next Dialogue`
  (`/Engine/EditorBlueprintResources/StandardMacros.IncrementInt` (`self.dialogueIndex`)
    (:`  `
      (if (== (`self.dialogueIndex`) (`KismetArrayLibrary.Array_Length` (`self.dialogueText`)))
        (`Widget.RemoveFromParent` (`self.DialogueGUI`))
        (`GameplayStatics.SetGamePaused` false)
        (`WidgetBlueprintLibrary.SetInputMode_GameOnly` (`GameplayStatics.GetPlayerController` 0))
        (set `self.isActive` false)
        (else
          (`TextBlock.SetText` (`/Game/GUI/wbp_dialogue.txt_dialogue` (`self.DialogueGUI`)) (`|GetArrayItem` (`self.dialogueText`) (`self.dialogueIndex`))))))))

(event `ChangeTextToDisplayKey`
  (bind _returnvalue (`EnhancedInputSubsystemInterface.QueryKeysMappedToAction` (pcsubsystem `EnhancedInputLocalPlayerSubsystem` (`GameplayStatics.GetPlayerController` 0)) (`self.InputToDisplay`)))
  (if (`KismetArrayLibrary.Array_IsEmpty` _returnvalue) :!label _label
    (`KismetSystemLibrary.DelayUntilNextTick`)
    (goto _label)
    (else
      (for _array_element _returnvalue
        (if (`KismetInputLibrary.Key_IsKeyboardKey` _array_element)
          (for (_array_element_2 _array_index) (`self.dialogueText`)
            (`KismetArrayLibrary.Array_Set` (`self.dialogueText`) _array_index (`KismetTextLibrary.Conv_StringToText` (`KismetStringLibrary.Replace` (`KismetTextLibrary.Conv_TextToString` _array_element_2) "[keyname]" (`KismetStringLibrary.Concat_StrStr` "[" (`KismetTextLibrary.Conv_TextToString` (`KismetInputLibrary.Key_GetDisplayName` _array_element)) "]")))))
          (break)))
      (bind _returnvalue_2 (`|CreateWidget` "/Game/GUI/wbp_dialogue.wbp_dialogue_C"))
      (bind _output_get (set `self.DialogueGUI` _returnvalue_2))
      (`TextBlock.SetText` (`/Game/GUI/wbp_dialogue.txt_dialogue` _output_get) (`|GetArrayItem` (`self.dialogueText`) (`self.dialogueIndex`))))))

(fn `UserConstructionScript`)