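; Level transition trigger that loads another level when the ZPlayer overlaps its box.
; It copies the player's gameplay timer into the game instance, then opens the level referenced by LevelToLoad.
; After the open call, it resets the player's checkpoint and last dialogue IDs and saves under the separately set LevelToSave name at checkpoint zero.
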(event `self.Box.OnComponentBeginOverlap`
  (params (OverlappedComponent :type "PrimitiveComponent Object Reference") (OtherActor :type "Actor Object Reference") (OtherComp :type "PrimitiveComponent Object Reference") (OtherBodyIndex :type Integer) (bFromSweep :type Boolean) (SweepResult :type "HitResult Structure (by ref)"))
  (bind _asbp_zplayer (cast `/Game/Characters/Blueprints/bp_ZPlayer` OtherActor))
  (bind _asbp_z_game_instance (cast `/Game/Misc/bp_zGameInstance` (`GameplayStatics.GetGameInstance`)))
  (set `/Game/Misc/bp_zGameInstance.gameplayTime` (`/Game/Entities/bp_gameplayTimer.TimerTime` (`/Game/Characters/Blueprints/bp_ZPlayer.Gameplay Timer` _asbp_zplayer)) _asbp_z_game_instance)
  (`GameplayStatics.OpenLevelBySoftObjectPtr` (`self.LevelToLoad`))
  (set `/Game/Characters/Blueprints/bp_ZPlayer.currentCheckpointID` 0 _asbp_zplayer)
  (set `/Game/Characters/Blueprints/bp_ZPlayer.lastDialogueActivated_ID` -1 _asbp_zplayer)
  (`/Game/Characters/Blueprints/bp_ZPlayer.Save With Set Data` _asbp_zplayer (`KismetStringLibrary.Conv_NameToString` (`self.LevelToSave`)) 0))

(fn `UserConstructionScript`)