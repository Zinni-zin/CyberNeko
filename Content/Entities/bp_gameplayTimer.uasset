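; Gameplay timer that counts elapsed time and can be started, stopped or reset.
; A timeline's playback position drives TimerTime, which is split each update into hours, minutes, seconds and hundredths (stored as Milliseconds).
; GetText and GetTimeAsString format these without zero padding, omitting leading empty units.
; UpdateTimeDiliation, when called, sets custom time dilation to the inverse of global dilation, offsetting slow or fast motion.
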(event `Start`
  (`TimelineComponent.SetNewTime` (`self.TimerTimeline`) (`self.TimerTime`))
  (`Timeline|TimerTimeline`
    (:`Update`
      (set `self.TimerTime` (`TimelineComponent.GetPlaybackPosition` (`self.TimerTimeline`)))
      (`self.Calculate Individual Time Components`))))

(event `Stop`
  (`TimelineComponent.Stop` (`self.TimerTimeline`)))

(event `Reset`
  (`self.Stop`)
  (set `self.TimerTime` 0.0)
  (`self.Start`))

(event `Calculate Individual Time Components`
  (bind _returnvalue (`KismetMathLibrary.FTrunc` (`self.TimerTime`)))
  (set `self.Hours` (/ _returnvalue 3600))
  (set `self.Minutes` (mod (/ _returnvalue 60) 60))
  (set `self.Seconds` (mod _returnvalue 60))
  (set `self.Milliseconds` (`KismetMathLibrary.FTrunc` (* (- (`self.TimerTime`) _returnvalue) 100.0))))

(event `Update Time Diliation`
  (set `self.CustomTimeDilation` (/ 1.0 (`GameplayStatics.GetGlobalTimeDilation`))))

(fn `Get Text`
  (returns (ReturnValue :type Text))
  (if (> (`self.Hours`) 0)
    (return (`KismetTextLibrary.Conv_StringToText` (`KismetStringLibrary.Concat_StrStr` (`KismetStringLibrary.Conv_IntToString` (`self.Hours`)) ":" (`KismetStringLibrary.Conv_IntToString` (`self.Minutes`)) ":" (`KismetStringLibrary.Conv_IntToString` (`self.Seconds`)) "." (`KismetStringLibrary.Conv_IntToString` (`self.Milliseconds`)))))
    (elif (> (`self.Minutes`) 0)
      (return (`KismetTextLibrary.Conv_StringToText` (`KismetStringLibrary.Concat_StrStr` (`KismetStringLibrary.Conv_IntToString` (`self.Minutes`)) ":" (`KismetStringLibrary.Conv_IntToString` (`self.Seconds`)) "." (`KismetStringLibrary.Conv_IntToString` (`self.Milliseconds`)))))
      (else
        (return (`KismetTextLibrary.Conv_StringToText` (`KismetStringLibrary.Concat_StrStr` (`KismetStringLibrary.Conv_IntToString` (`self.Seconds`)) "." (`KismetStringLibrary.Conv_IntToString` (`self.Milliseconds`)))))))))

(fn `Get Time as String`
  (returns (ReturnValue :type String))
  (if (> (`self.Hours`) 0)
    (return (`KismetStringLibrary.Concat_StrStr` (`KismetStringLibrary.Conv_IntToString` (`self.Hours`)) ":" (`KismetStringLibrary.Conv_IntToString` (`self.Minutes`)) ":" (`KismetStringLibrary.Conv_IntToString` (`self.Seconds`)) "." (`KismetStringLibrary.Conv_IntToString` (`self.Milliseconds`))))
    (elif (> (`self.Minutes`) 0)
      (return (`KismetStringLibrary.Concat_StrStr` (`KismetStringLibrary.Conv_IntToString` (`self.Minutes`)) ":" (`KismetStringLibrary.Conv_IntToString` (`self.Seconds`)) "." (`KismetStringLibrary.Conv_IntToString` (`self.Milliseconds`))))
      (else
        (return (`KismetStringLibrary.Concat_StrStr` (`KismetStringLibrary.Conv_IntToString` (`self.Seconds`)) "." (`KismetStringLibrary.Conv_IntToString` (`self.Milliseconds`))))))))

(fn `UserConstructionScript`)