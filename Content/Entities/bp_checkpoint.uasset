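; Checkpoint actor that registers itself as the current checkpoint of a bp_ZPlayer touching its trigger.
; Both begin and end overlap set the player's CurrentCheckpoint, with IsActivated latching it so it registers only once.
; The construction script converts the local spawn location to world space.
; Save-game calls storing level, checkpoint ID and rewind time limit are present but disconnected, so nothing is saved here.
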(event `self.Trigger.OnComponentBeginOverlap`
  (params (OverlappedComponent :type "PrimitiveComponent Object Reference") (OtherActor :type "Actor Object Reference") (OtherComp :type "PrimitiveComponent Object Reference") (OtherBodyIndex :type Integer) (bFromSweep :type Boolean) (SweepResult :type "HitResult Structure (by ref)"))
  (if (not (`self.isActivated`))
    (bind _asbp_zplayer (cast `/Game/Characters/Blueprints/bp_ZPlayer` OtherActor))
    (set `/Game/Characters/Blueprints/bp_ZPlayer.currentCheckpoint` self _asbp_zplayer)
    (set `self.isActivated` true)))

(event `self.Trigger.OnComponentEndOverlap`
  (params (OverlappedComponent :type "PrimitiveComponent Object Reference") (OtherActor :type "Actor Object Reference") (OtherComp :type "PrimitiveComponent Object Reference") (OtherBodyIndex :type Integer))
  (if (not (`self.isActivated`))
    (bind _asbp_zplayer (cast `/Game/Characters/Blueprints/bp_ZPlayer` OtherActor))
    (set `/Game/Characters/Blueprints/bp_ZPlayer.currentCheckpoint` self _asbp_zplayer)
    (set `self.isActivated` true)))

(fn `UserConstructionScript`
  (set `self.checkpointSpawnLocationWorld` (`KismetMathLibrary.TransformLocation` (`self.GetTransform`) (`self.CheckpointSpawnLocation`))))