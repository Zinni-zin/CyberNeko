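; Collapsing trap platform that shatters a geometry collection when the player overlaps its trigger, then fades out and destroys itself.
; On overlap it removes an optional attached volume, enables physics, activates the player's damage field, sets jump permission and destroys the trigger.
; A timeline drives the material Fade parameter; below half it stops the damage field and flips jump permission back.
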(event `self.ReceiveBeginPlay`)

(event `self.Trap Trigger.OnComponentBeginOverlap`
  (params (OverlappedComponent :type "PrimitiveComponent Object Reference") (OtherActor :type "Actor Object Reference") (OtherComp :type "PrimitiveComponent Object Reference") (OtherBodyIndex :type Integer) (bFromSweep :type Boolean) (SweepResult :type "HitResult Structure (by ref)"))
  (bind _asbp_zplayer (cast `/Game/Characters/Blueprints/bp_ZPlayer` OtherActor))
  (bind _attached_volume_to_remove (`self.attached volume to remove`)
    (:`then`
      (`self.K2_DestroyActor` _attached_volume_to_remove))
    (:`else`
      _))
  (`PrimitiveComponent.SetSimulatePhysics` (`self.GeometryCollection`) true)
  (set `/Game/Characters/Blueprints/bp_ZPlayer.damageFieldScale` (`self.damageFieldScale`) _asbp_zplayer)
  (`self.SetActorTickEnabled` _asbp_zplayer true)
  (`/Game/Characters/Blueprints/bp_ZPlayer.ActivateDamage Field` _asbp_zplayer)
  (set `/Game/Characters/Blueprints/bp_ZPlayer.canPlayerJump` (not (`self.canPreventPlayerFromJumping`)) _asbp_zplayer)
  (`ActorComponent.K2_DestroyComponent` (`self.Trap Trigger`))
  (`TimelineComponent.SetPlayRate` (`self.FadeTimeline`) (`self.timelinePlayRate`))
  (bind (_direction _fadetrack) (`Timeline|FadeTimeline`)
    (:`Update`
      (`MeshComponent.SetScalarParameterValueOnMaterials` (`self.GeometryCollection`) "Fade" _fadetrack)
      (if (< _fadetrack 0.5)
        (set `/Game/Characters/Blueprints/bp_ZPlayer.canPlayerJump` (`self.canPreventPlayerFromJumping`) _asbp_zplayer)
        (`/Game/Characters/Blueprints/bp_ZPlayer.StopDamageField` _asbp_zplayer)))
    (:`Finished`
      (`/Game/Characters/Blueprints/bp_ZPlayer.StopDamageField` _asbp_zplayer)
      (`self.K2_DestroyActor`))))

(fn `UserConstructionScript`)