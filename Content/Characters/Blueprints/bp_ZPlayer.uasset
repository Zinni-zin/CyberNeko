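; Player character for a platformer with time powers: rewind, slowing of moving platforms, and global speed-up.
; Enhanced Input drives movement, sprint, jump, dive, pause and interface-based interaction, with several moves gated by ability flags.
; Ladders use a timeline snap and flying mode, ropes attach the character, and sprint speed feeds the wall-run component.
; BeginPlay builds widgets and restores checkpoint, rewind limit and abilities from the save, granting all abilities on TestingMap.
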(event `self.ReceiveTick`
  (params (DeltaSeconds :type "Float (single-precision)"))
  (bind (_returnvalue_x _returnvalue_y) (`KismetMathLibrary.BreakVector2D` (`|GetInputActionValue`)))
  (bind _returnvalue (`SceneComponent.K2_GetComponentLocation` (`self.legLineTrace`)))
  (if (and (`self.isOnLadder`) (< _returnvalue_y 0.0))
    (bind (_outhit _returnvalue_2) (`KismetSystemLibrary.LineTraceSingle` :`Start` _returnvalue :`End` (+ _returnvalue (* (`self.GetActorUpVector`) -10.0)) :`TraceChannel` "TraceTypeQuery1" :`DrawDebugType` "ForOneFrame"))
    (if _returnvalue_2
      (`self.toggleClimbing` false))))

(event `self.ReceiveBeginPlay`
  (`|ExecutionSequence`
    (:`then_0`
      (set `C_WallRun.m_wallRunSpeed` (`CharacterMovementComponent.MaxWalkSpeed` (`self.CharacterMovement`)) (`self.wallRunComp`)))
    (:`then_1`
      (bind _asplayer_controller (cast `PlayerController` (`self.GetController`)))
      (bind _returnvalue (pcsubsystem `EnhancedInputLocalPlayerSubsystem` _asplayer_controller))
      (`/Engine/EditorBlueprintResources/StandardMacros.IsValid` _returnvalue
        (:`Is Valid`
          (if (not (`.ReturnValue` (`EnhancedInputSubsystemInterface.HasMappingContext` _returnvalue "/Game/Input/imc_Basic.imc_Basic")))
            (`EnhancedInputSubsystemInterface.AddMappingContext` _returnvalue "/Game/Input/imc_Basic.imc_Basic" 0 (struct))))))
    (:`then_2`
      (`|ExecutionSequence`
        (:`then_0`
          (bind _returnvalue_2 (`|CreateWidget` "/Game/GUI/Time/wbp_timer.wbp_timer_C"))
          (set `self.TimerWidget` _returnvalue_2)
          (set `/Game/GUI/Time/wbp_timer.player` self _returnvalue_2)
          (`UserWidget.AddToViewport` _returnvalue_2 0))
        (:`then_1`
          (bind _returnvalue_3 (`|CreateWidget` "/Game/GUI/Menus/wbp_pauseMenu.wbp_pauseMenu_C"))
          (bind _output_get (set `self.pauseMenuWidget` _returnvalue_3))
          (`UserWidget.AddToViewport` _output_get 5)
          (set `Widget.Visibility` "Hidden" _returnvalue_3)
          (set `/Game/GUI/Menus/wbp_pauseMenu.player` self _returnvalue_3)
          (`/Game/GUI/Menus/wbp_pauseMenu.SetPlayerMouseInvertY` _returnvalue_3))))
    (:`then_3`
      (bind _asbp_z_game_instance (cast `/Game/Misc/bp_zGameInstance` (`GameplayStatics.GetGameInstance`)))
      (bind _currentfilename (`/Game/Misc/bp_zGameInstance.currentFileName` _asbp_z_game_instance))
      (bind _returnvalue_4 (`GameplayStatics.DoesSaveGameExist` _currentfilename))
      (if _returnvalue_4
        (bind _returnvalue_5 (`GameplayStatics.LoadGameFromSlot` _currentfilename))
        (bind _asbpsg_save_game (cast `/Game/Misc/bpsg_saveGame` _returnvalue_5))
        (bind _output_get_2 (set `self.SaveGame` _asbpsg_save_game))
        (bind _outactors (`GameplayStatics.GetAllActorsOfClass` "/Game/Entities/bp_checkpoint.bp_checkpoint_C"))
        (for _array_element _outactors
          (if (== (`/Game/Entities/bp_checkpoint.Id` _array_element) (`/Game/Misc/bpsg_saveGame.CheckpointID` _output_get_2))
            (set `self.currentCheckpoint` _array_element)
            (break)))
        (`self.ChangeTimerLimit` (`/Game/Misc/bpsg_saveGame.timeRewindLimit` _output_get_2))
        (`self.ChangeAbilityFlag` (`/Game/Misc/bpsg_saveGame.AbilityFlags` _output_get_2))
        (`self.OnReset`)
        (else
          (bind _returnvalue_6 (`GameplayStatics.CreateSaveGameObject` "/Game/Misc/bpsg_saveGame.bpsg_saveGame_C"))
          (set `self.SaveGame` _returnvalue_6))))
    (:`then_4`
      (bind _returnvalue_7 (`GameplayStatics.GetCurrentLevelName` true))
      (if (== _returnvalue_7 "TestingMap")
        (`self.AddAllAbilityFlags`)))))

(event `EnhancedInput|/Game/Input/Actions/ia_move`
  (params (ActionValue :type "Vector2D Structure") (ElapsedSeconds :type "Float (double-precision)") (TriggeredSeconds :type "Float (double-precision)") (InputAction :type "InputAction Object Reference" :default "/Game/Input/Actions/ia_move.ia_move"))
  (bind (_returnvalue_roll _returnvalue_pitch _returnvalue_yaw) (`KismetMathLibrary.BreakRotator` (`self.GetControlRotation`)))
  (:`Triggered`
    (if (`self.isRewinding`)
      _
      (elif (`self.m_isDiving`)
        _
        (elif (`self.isOnLadder`)
          (`self.AddMovementInput` (`KismetMathLibrary.GetUpVector` (`KismetMathLibrary.MakeRotator` 0.0 0.0 _returnvalue_yaw)) ActionValue_Y)
          (else
            (`self.MoveHoriz` ActionValue_X)
            (`self.MoveFAB` ActionValue_Y)))))))

(event `EnhancedInput|/Game/Input/Actions/ia_look`
  (params (ActionValue :type "Vector2D Structure") (ElapsedSeconds :type "Float (double-precision)") (TriggeredSeconds :type "Float (double-precision)") (InputAction :type "InputAction Object Reference" :default "/Game/Input/Actions/ia_look.ia_look"))
  (:`Triggered`
    (`self.AddControllerYawInput` ActionValue_X)
    (if (`self.isCamInvertedY`)
      (`self.AddControllerPitchInput` ActionValue_Y)
      (else
        (`self.AddControllerPitchInput` (* -1.0 ActionValue_Y))))))

(event `EnhancedInput|/Game/Input/Actions/ia_sprint`
  (params (ActionValue :type Boolean) (ElapsedSeconds :type "Float (double-precision)") (TriggeredSeconds :type "Float (double-precision)") (InputAction :type "InputAction Object Reference" :default "/Game/Input/Actions/ia_sprint.ia_sprint"))
  (:`Triggered`
    (bind _returnvalue (`self.HasAbilityFlag` "CanSprint"))
    (if (and _returnvalue (not (`self.isRewinding`)) (not (`self.m_isDiving`)))
      (bind _output_get (set `CharacterMovementComponent.MaxWalkSpeed` (`self.sprintSpeed`) (`self.CharacterMovement`)))
      (set `C_WallRun.m_wallRunSpeed` _output_get (`self.wallRunComp`))))
  (:`Canceled`
    (bind _output_get_2 (set `CharacterMovementComponent.MaxWalkSpeed` (`self.runSpeed`) (`self.CharacterMovement`) :!label _label))
    (set `C_WallRun.m_wallRunSpeed` _output_get_2 (`self.wallRunComp`)))
  (:`Completed`
    (goto _label)))

(event `EnhancedInput|/Game/Input/Actions/ia_jump`
  (params (ActionValue :type Boolean) (ElapsedSeconds :type "Float (double-precision)") (TriggeredSeconds :type "Float (double-precision)") (InputAction :type "InputAction Object Reference" :default "/Game/Input/Actions/ia_jump.ia_jump"))
  (:`Triggered`
    (bind _returnvalue (`self.HasAbilityFlag` "CanJump"))
    (if _returnvalue
      (if (`self.isRewinding`)
        _
        (elif (and (`self.m_isDiving`) (`self.isJumping`))
          _
          (elif (`self.canPlayerJump`)
            (`self.CharJump`)
            (set `self.isJumping` true))))))
  (:`Completed`
    (`self.StopJumping`)
    (set `self.isJumping` false)))

(event `EnhancedInput|/Game/Input/Actions/ia_dive`
  (params (ActionValue :type Boolean) (ElapsedSeconds :type "Float (double-precision)") (TriggeredSeconds :type "Float (double-precision)") (InputAction :type "InputAction Object Reference" :default "/Game/Input/Actions/ia_dive.ia_dive"))
  (:`Triggered`
    (bind _returnvalue (`self.HasAbilityFlag` "CanDive"))
    (if _returnvalue
      (if (`self.isRewinding`)
        _
        (elif (not (`self.m_isDiving`))
          (`self.Dive`))))))

(event `EnhancedInput|/Game/Input/Actions/ia_pause`
  (params (ActionValue :type Boolean) (ElapsedSeconds :type "Float (double-precision)") (TriggeredSeconds :type "Float (double-precision)") (InputAction :type "InputAction Object Reference" :default "/Game/Input/Actions/ia_pause.ia_pause"))
  (bind _returnvalue (`GameplayStatics.GetPlayerController` 0))
  (bind _pausemenuwidget (`self.pauseMenuWidget`))
  (:`Started`
    (if (not (`self.isPaused`))
      (set `Widget.Visibility` "Visible" _pausemenuwidget)
      (`GameplayStatics.SetGamePaused` true)
      (set `PlayerController.bShowMouseCursor` true _returnvalue)
      (`WidgetBlueprintLibrary.SetInputMode_GameAndUIEx` _returnvalue (`self.pauseMenuWidget`))
      (set `self.isPaused` true)
      (else
        (set `Widget.Visibility` "Hidden" _pausemenuwidget)
        (`GameplayStatics.SetGamePaused` false)
        (set `PlayerController.bShowMouseCursor` false _returnvalue)
        (`WidgetBlueprintLibrary.SetInputMode_GameOnly` _returnvalue)
        (set `self.isPaused` false)
        (bind _aswbp_pause_menu (cast `/Game/GUI/Menus/wbp_pauseMenu` (`self.pauseMenuWidget`)))
        (`/Game/GUI/Menus/wbp_pauseMenu.SetPlayerMouseInvertY` _aswbp_pause_menu)))))

(event `EnhancedInput|/Game/Input/Actions/ia_interact`
  (params (ActionValue :type Boolean) (ElapsedSeconds :type "Float (double-precision)") (TriggeredSeconds :type "Float (double-precision)") (InputAction :type "InputAction Object Reference" :default "/Game/Input/Actions/ia_interact.ia_interact"))
  (:`Started`
    (`|ExecutionSequence`
      (:`then_0`
        (if (`self.isOnLadder`)
          (set `self.isOnLadder` false)
          (`CharacterMovementComponent.SetMovementMode` (`self.CharacterMovement`) "MOVE_Walking" 0)))
      (:`then_1`
        (for _array_element (`self.GetOverlappingActors` "/Script/Engine.Actor")
          (if (`KismetSystemLibrary.DoesImplementInterface` _array_element "/Script/CyberNeko.CharacterActions")
            (message `CharacterActions.CharInteracted` _array_element)
            (break)))))))

(event `OnLadderSnap`
  (bind (_actorlocationbeforeladderclimb_x _actorlocationbeforeladderclimb_y _actorlocationbeforeladderclimb_z) (`KismetMathLibrary.BreakVector` (`self.ActorLocationBeforeLadderClimb`)))
  (bind (_returnvalue_x _returnvalue_y) (`KismetMathLibrary.BreakVector` (`SceneComponent.K2_GetComponentLocation` (`/Game/Entities/bp_ladder.ladderClimbOffset` (`self.currentLadderRef`)))))
  (set `self.ActorLocationBeforeLadderClimb` (`self.K2_GetActorLocation`))
  (set `self.ActorRotationBeforeLadderClimb` (`self.K2_GetActorRotation`))
  (bind (_direction _snapalpha) (`Timeline|LadderSnapAnimationTimeline`)
    (:`Update`
      (`self.K2_SetActorLocationAndRotation` (`KismetMathLibrary.VLerp` (`self.ActorLocationBeforeLadderClimb`) (`KismetMathLibrary.MakeVector` _returnvalue_x _returnvalue_y _actorlocationbeforeladderclimb_z) _snapalpha) (`KismetMathLibrary.RLerp` (`self.ActorRotationBeforeLadderClimb`) (`KismetMathLibrary.Conv_VectorToRotator` (* (`self.GetActorForwardVector` (`self.currentLadderRef`)) -1.0)) _snapalpha true)))))

(event `self.CharGrabbedRope`
  (params (rope :type "Object Object Reference"))
  (if (and (`self.canAttachToRope`) (not (`self.isRewinding`)))
    (`CharacterMovementComponent.SetMovementMode` (`self.CharacterMovement`) "MOVE_None" 0)
    (set `self.defaultRotation` (`self.K2_GetActorRotation` self))
    (set `self.isSwinging` true)
    (bind _asbp_rope (cast `/Game/Entities/bp_rope` rope))
    (set `self.RopeGrabbedOnto` _asbp_rope)
    (`self.K2_AttachToComponent` (`/Game/Entities/bp_rope.RopeEnd` _asbp_rope) "None" "SnapToTarget" "KeepWorld" "KeepWorld")))

(event `OnReset`
  (bind _currentcheckpoint (`self.currentCheckpoint`))
  (`/Engine/EditorBlueprintResources/StandardMacros.IsValid` _currentcheckpoint
    (:`Is Valid`
      (`self.K2_SetActorTransform` (`KismetMathLibrary.MakeTransform` (`/Game/Entities/bp_checkpoint.checkpointSpawnLocationWorld` _currentcheckpoint) (`self.K2_GetActorRotation` _currentcheckpoint)) false true)
      (`self.ResetTimeRewind`))))

(event `EnhancedInput|/Game/Input/Actions/ia_rewind`
  (params (ActionValue :type Boolean) (ElapsedSeconds :type "Float (double-precision)") (TriggeredSeconds :type "Float (double-precision)") (InputAction :type "InputAction Object Reference" :default "/Game/Input/Actions/ia_rewind.ia_rewind"))
  (:`Triggered`
    (if (not (`self.isRewinding`))
      (`self.StartRewind`)
      (set `self.isRewinding` true)))
  (:`Completed`
    (`self.StopRewind`)
    (set `self.isRewinding` false)))

(event `EnhancedInput|/Game/Input/Actions/ia_slowTime`
  (params (ActionValue :type Boolean) (ElapsedSeconds :type "Float (double-precision)") (TriggeredSeconds :type "Float (double-precision)") (InputAction :type "InputAction Object Reference" :default "/Game/Input/Actions/ia_slowTime.ia_slowTime"))
  (:`Started`
    (bind _returnvalue (`self.HasAbilityFlag` "CanSlowTime"))
    (if _returnvalue
      (bind _outactors (`GameplayStatics.GetAllActorsOfClass` "/Game/Entities/bp_MovingPlatform.bp_MovingPlatform_C"))
      (for _array_element _outactors
        (`/Game/Entities/bp_MovingPlatform.SetSlowMo` _array_element (`self.SlowmoFactor`)))))
  (:`Completed`
    (bind _outactors_2 (`GameplayStatics.GetAllActorsOfClass` "/Game/Entities/bp_MovingPlatform.bp_MovingPlatform_C"))
    (for _array_element_2 _outactors_2
      (`/Game/Entities/bp_MovingPlatform.SetSlowMo` _array_element_2 1.0))))

(event `EnhancedInput|/Game/Input/Actions/ia_speedTime`
  (params (ActionValue :type Boolean) (ElapsedSeconds :type "Float (double-precision)") (TriggeredSeconds :type "Float (double-precision)") (InputAction :type "InputAction Object Reference" :default "/Game/Input/Actions/ia_speedTime.ia_speedTime"))
  (:`Triggered`
    (if (not (`self.isRewinding`))
      (`GameplayStatics.SetGlobalTimeDilation` 2.0)))
  (:`Canceled`
    (`GameplayStatics.SetGlobalTimeDilation` 1.0 :!label _label))
  (:`Completed`
    (goto _label)))

(fn `ActivateDamage Field`
  (bind (_returnvalue_location _returnvalue_rotation _returnvalue_scale) (`KismetMathLibrary.BreakTransform` (`SceneComponent.GetSocketTransform` (`self.Mesh`) "feetDamage" "RTS_World")))
  (`/Engine/EditorBlueprintResources/StandardMacros.DoOnce` false
    (:`Completed`
      (bind _returnvalue (`|SpawnActorFromClass` "/Game/Chaos/CollapsingPlatforms/bp_damage_masterField.bp_damage_masterField_C" (`KismetMathLibrary.MakeTransform` _returnvalue_location _returnvalue_rotation (* _returnvalue_scale (`self.damageFieldScale`))) "Undefined" "OverrideRootScale" null null))
      (bind _output_get (set `self.damageField` _returnvalue))
      (`self.K2_AttachToComponent` _output_get (`self.Mesh`) "feetDamage" "SnapToTarget" "SnapToTarget" "KeepWorld" true)
      (`/Engine/EditorResources/FieldNodes/FS_MasterField.CE_Trigger` (`self.damageField`)))))

(fn `AddAllAbilityFlags`
  (`self.SetAbilityFlag` "CanJump")
  (`self.SetAbilityFlag` "CanSprint")
  (`self.SetAbilityFlag` "CanDive")
  (`self.SetAbilityFlag` "CanWallRun")
  (`self.SetAbilityFlag` "CanSlowTime")
  (`self.SetAbilityFlag` "CanSpeedTime"))

(fn `Save`
  (locals (checkpointID :type Integer))
  (bind _currentcheckpoint (`self.currentCheckpoint`))
  (`/Engine/EditorBlueprintResources/StandardMacros.IsValid` (`self.SaveGame`)
    (:`Is Valid`
      _)
    (:`Is Not Valid`
      (bind _returnvalue (`GameplayStatics.CreateSaveGameObject` "/Game/Misc/bpsg_saveGame.bpsg_saveGame_C"))
      (set `self.SaveGame` _returnvalue)))
  (bind _asbp_z_game_instance (cast `/Game/Misc/bp_zGameInstance` (`GameplayStatics.GetGameInstance`)))
  (bind _returnvalue_2 (`GameplayStatics.GetCurrentLevelName` true))
  (`/Engine/EditorBlueprintResources/StandardMacros.IsValid` _currentcheckpoint
    (:`Is Valid`
      (set `local.checkpointID` (`/Game/Entities/bp_checkpoint.Id` _currentcheckpoint)))
    (:`Is Not Valid`
      _))
  (`/Game/Misc/bpsg_saveGame.Save` (`self.SaveGame`) _returnvalue_2 (`local.checkpointID`) (`self.getRewindTimeLimit`) (`self.m_abilityFlags`) (`/Game/Misc/bp_zGameInstance.currentFileName` _asbp_z_game_instance)))

(fn `StopDamageField`
  (bind _damagefield (`self.damageField`))
  (`self.SetActorTickEnabled` self false)
  (`/Engine/EditorBlueprintResources/StandardMacros.IsValid` _damagefield
    (:`Is Valid`
      (`self.K2_DestroyActor` _damagefield)
      (set `self.damageField` null))))

(fn `StopSwing`
  (locals (velBeforeLaunch :type "Vector Structure"))
  (bind (_returnvalue_roll _returnvalue_pitch _returnvalue_yaw) (`KismetMathLibrary.BreakRotator` (`self.K2_GetActorRotation`)))
  (bind _ropegrabbedonto (`self.RopeGrabbedOnto`))
  (bind (_defaultrotation_roll _defaultrotation_pitch) (`KismetMathLibrary.BreakRotator` (`self.defaultRotation`)))
  (`CharacterMovementComponent.SetMovementMode` (`self.CharacterMovement`) "MOVE_Falling" 0)
  (set `self.isSwinging` false)
  (set `self.isSwingingForward` false)
  (set `self.isSwingingBackward` false)
  (`self.K2_DetachFromActor` self "KeepWorld" "KeepRelative" "KeepWorld")
  (`self.K2_SetActorRotation` (`KismetMathLibrary.MakeRotator` _defaultrotation_roll _defaultrotation_pitch (- _returnvalue_yaw 90.0)))
  (`/Engine/EditorBlueprintResources/StandardMacros.IsValid` _ropegrabbedonto
    (:`Is Valid`
      (`CharacterMovementComponent.AddImpulse` (`self.CharacterMovement`) (/ (* (`SceneComponent.GetComponentVelocity` (`/Game/Entities/bp_rope.RopeEnd` _ropegrabbedonto)) (`self.swingImpulse`)) (`self.swingImpulseFactor`)) false)
      (set `self.canAttachToRope` false))))

(fn `toggleClimbing`
  (params (isClimbing :type Boolean) (ladder :type "/Game/Entities/bp_ladder Object Reference"))
  (set `self.currentLadderRef` ladder)
  (bind _output_get (set `self.isOnLadder` isClimbing))
  (if _output_get
    (`CharacterMovementComponent.SetMovementMode` (`self.CharacterMovement`) "MOVE_Flying" 0)
    (set `CharacterMovementComponent.bOrientRotationToMovement` false (`self.CharacterMovement`))
    (`self.OnLadderSnap`)
    (else
      (`CharacterMovementComponent.SetMovementMode` (`self.CharacterMovement`) "MOVE_Walking" 0)
      (set `CharacterMovementComponent.bOrientRotationToMovement` true (`self.CharacterMovement`)))))

(fn `UserConstructionScript`)